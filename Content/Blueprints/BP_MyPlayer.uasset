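; Player Blueprint that drives the game's UI flow: main menu, crosshair HUD, pause menu and death screen.
; A ShowPage helper creates and displays each widget, while events toggle input mode, mouse cursor and controller rotation between menus and gameplay.
; BeginPlay activates an intro camera behind the menu, and GameStarted activates the gameplay camera.
; UpdateHUDHealth forwards health changes to the crosshair widget's health bar.
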(event `EnhancedInput|/Game/Inputs/IA_Pause`
  (params (ActionValue :type Boolean) (ElapsedSeconds :type "Float (double-precision)") (TriggeredSeconds :type "Float (double-precision)") (InputAction :type "InputAction Object Reference" :default "/Game/Inputs/IA_Pause.IA_Pause"))
  (bind _returnvalue (`GameplayStatics.GetPlayerController` 0))
  ;[0.15 0.15 0.15 0.5 42] Pause
  (:`Triggered`
    (if (`self.isPause`)
      (`Widget.SetVisibility` (stale _valuewidget) "Hidden" :!label _label)
      (set `self.isPause` false)
      (`GameplayStatics.SetGamePaused` false)
      (`WidgetBlueprintLibrary.SetInputMode_GameOnly` _returnvalue)
      (set `self.bUseControllerRotationPitch` true)
      (set `self.bUseControllerRotationYaw` true)
      (set `PlayerController.bShowMouseCursor` false _returnvalue)
      (else
        (bind _valuewidget (`self.ShowPage` "/Game/UI/WB_Pause.WB_Pause_C"))
        (set `self.isPause` true)
        (`GameplayStatics.SetGamePaused` true)
        (set `self.bUseControllerRotationPitch` false)
        (set `self.bUseControllerRotationYaw` false)
        (set `PlayerController.bShowMouseCursor` true _returnvalue)
        (`WidgetBlueprintLibrary.SetInputMode_UIOnlyEx` _returnvalue null)))))

(event `Pause`
  ;[0.15 0.15 0.15 0.5 42] Pause
  (goto _label))

(event `self.ShowGameOverScreen`
  (bind _returnvalue (`GameplayStatics.GetPlayerController` 0))
  ;[0.15 0.15 0.15 0.5 42] GameOverScreen
  (`self.ShowPage` "/Game/UI/WB_Death.WB_Death_C")
  (`Widget.SetVisibility` (stale `GameStarted` _valuewidget) "Hidden")
  (set `self.bUseControllerRotationPitch` false)
  (set `self.bUseControllerRotationYaw` false)
  (set `PlayerController.bShowMouseCursor` true _returnvalue)
  (`WidgetBlueprintLibrary.SetInputMode_UIOnlyEx` _returnvalue null))

(event `self.ReceiveBeginPlay`
  (bind _returnvalue (`GameplayStatics.GetPlayerController` 0))
  ;[0.15 0.15 0.15 0.5 42] BeginPlay - Menu
  (`ActorComponent.SetActive` (`self.CameraDebutGame`) true false)
  (bind _valuewidget (`self.ShowPage` "/Game/UI/WB_MainMenu.WB_MainMenu_C"))
  (`self.ShowPage` null)
  (set `self.bUseControllerRotationPitch` false)
  (set `self.bUseControllerRotationYaw` false)
  (set `PlayerController.bShowMouseCursor` true _returnvalue)
  (`WidgetBlueprintLibrary.SetInputMode_UIOnlyEx` _returnvalue null))

(event `GameStarted`
  (bind _returnvalue (`GameplayStatics.GetPlayerController` 0))
  ;[0.15 0.15 0.15 0.5 42] Lancer la partie
  (`ActorComponent.SetActive` (`self.Camera`) true false)
  (bind _valuewidget (`self.ShowPage` "/Game/UI/WB_Crosshair.WB_Crosshair_C"))
  (`WidgetBlueprintLibrary.SetInputMode_GameOnly` _returnvalue)
  (set `PlayerController.bShowMouseCursor` false _returnvalue)
  (set `self.bUseControllerRotationPitch` true)
  (set `self.bUseControllerRotationYaw` true)
  (`Widget.SetVisibility` (stale `self.ReceiveBeginPlay` _valuewidget) "Hidden"))

(event `self.UpdateHUDHealth`
  (params (NewHealth :type "Float (single-precision)"))
  ;[0.15 0.15 0.15 0.5 42] Update ATH
  (bind _aswb_crosshair (cast `/Game/UI/WB_Crosshair` (stale `GameStarted` _valuewidget)))
  (`/Game/UI/WB_Crosshair.UpdateHealthBar` _aswb_crosshair NewHealth))

(fn `ShowPage`
  (params (NewParam :type "UserWidget Class Reference"))
  (returns (ValueWidget :type "UserWidget Object Reference"))
  (bind _returnvalue (`|CreateWidget` NewParam))
  (`UserWidget.AddToViewport` _returnvalue 0)
  (return _returnvalue))

(fn `UserConstructionScript`)